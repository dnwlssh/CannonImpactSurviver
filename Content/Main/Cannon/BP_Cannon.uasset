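; BP_Cannon is a cannon actor that automatically fires BP_CannonBall projectiles.
; On BeginPlay, a looping timer spawns one ball at the LaunchDirection component's world transform every few seconds.
; A second looping timer raises ProjectileCount up to MaxProjectileCount as a difficulty ramp.
; That count does not affect firing, as the loop that reads it is disconnected and empty.
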(event Custom|FIre
  (Game|SpawnActorfromClass "/Game/Main/Cannon/CannonBall/BP_CannonBall.BP_CannonBall_C" (Transformation|GetWorldTransform (Variables|Default|GetLaunchDirection)) "Undefined" "MultiplyWithRoot" 0 0))

(event Custom|IncreaseDifficulty
  (if (< (Variables|Default|GetProjectileCount) (Variables|Default|GetMaxProjectileCount))
    (Variables|Default|SetProjectileCount (+ (Variables|Default|GetProjectileCount) 1.0))))

(event EventBeginPlay
  (Utilities|Time|SetTimerbyEvent (delegate Custom|FIre) 3.0 true)
  (Utilities|Time|SetTimerbyEvent (delegate Custom|IncreaseDifficulty) 5.0 true))

(fn ConstructionScript)
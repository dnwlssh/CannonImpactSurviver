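; BP_CannonBall is a cannonball actor that explodes on contact and damages the player.
; Sphere overlap and actor Hit share one path that applies fixed damage to player pawn 0, whatever was struck, and spawns a Niagara explosion at the ball's location.
; It then disables the sphere's collision, hides it and destroys the actor after a short delay.
; The HasExplode setter is unconnected, so no flag guards against repeat triggers.
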(event OnComponentBeginOverlap(Sphere)
  (params (OverlappedComponent :type Primitive%20Component%20Object%20Reference) (OtherActor :type Actor%20Object%20Reference) (OtherComp :type Primitive%20Component%20Object%20Reference) (OtherBodyIndex :type Integer) (bFromSweep :type Boolean) (SweepResult :type Hit%20Result%20Structure%20%28by%20ref%29))
  (Game|Damage|ApplyDamage (Game|Player|GetPlayerPawn 0) 2e+01 0 0)
  (Niagara|SpawnSystematLocation "/Game/Fab/Fire_EXP_Vol01_Free/Niagara/EXP/NS_Sub_EXP_Mid_002_02.NS_Sub_EXP_Mid_002_02" (Transformation|GetActorLocation))
  (Collision|SetCollisionEnabled (Variables|Default|GetSphere) "NoCollision")
  (Development|SetHiddeninGame (Variables|Default|GetSphere) true false)
  (Utilities|FlowControl|Delay 0.2)
  (Actor|DestroyActor))

(event EventBeginPlay)

(event Collision|EventActorBeginOverlap
  (params (OtherActor :type Actor%20Object%20Reference)))

(event EventTick
  (params (DeltaSeconds :type Float%20%28single-precision%29)))

(event Collision|EventHit
  (params (MyComp :type Primitive%20Component%20Object%20Reference) (Other :type Actor%20Object%20Reference) (OtherComp :type Primitive%20Component%20Object%20Reference) (bSelfMoved :type Boolean) (HitLocation :type Vector :default "0, 0, 0") (HitNormal :type Vector :default "0, 0, 0") (NormalImpulse :type Vector :default "0, 0, 0") (Hit :type Hit%20Result%20Structure%20%28by%20ref%29))
  (Game|Damage|ApplyDamage (Game|Player|GetPlayerPawn 0) 2e+01 0 0)
  (Niagara|SpawnSystematLocation "/Game/Fab/Fire_EXP_Vol01_Free/Niagara/EXP/NS_Sub_EXP_Mid_002_02.NS_Sub_EXP_Mid_002_02" (Transformation|GetActorLocation))
  (Collision|SetCollisionEnabled (Variables|Default|GetSphere) "NoCollision")
  (Development|SetHiddeninGame (Variables|Default|GetSphere) true false)
  (Utilities|FlowControl|Delay 0.2)
  (Actor|DestroyActor))

(fn ConstructionScript)